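; Transmitter actor that teleports the player pawn to another Transmitter in the level.
; Any overlap on its TriggerBox sets IsActive, with no actor filter or end-overlap reset.
; ActivateTransmitter requires IsInUse and IsActive, moves the pawn just above the destination, then clears both flags.
; The destination is picked by indexing GetAllActorsOfClass with DestinationTransmitter, so it depends on that array's order.
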(event `ActivateTransmitter`
  (if (and (`self.isInUse`) (stale `self.TriggerBox.OnComponentBeginOverlap` _output_get))
    (bind _outactors (`GameplayStatics.GetAllActorsOfClass` "Transmitter_C"))
    (`self.K2_SetActorLocation` (`GameplayStatics.GetPlayerPawn` 0) (+ (`self.K2_GetActorLocation` (`|GetArrayItem` _outactors (`self.DestinationTransmitter`))) (0.0 0.0 1.0)) false true)
    (set `self.isInUse` false)
    (set `self.isActive` false)))

(event `self.TriggerBox.OnComponentBeginOverlap`
  (params (OverlappedComponent :type "PrimitiveComponent Object Reference") (OtherActor :type "Actor Object Reference") (OtherComp :type "PrimitiveComponent Object Reference") (OtherBodyIndex :type Integer) (bFromSweep :type Boolean) (SweepResult :type "HitResult Structure (by ref)"))
  (bind _output_get (set `self.isActive` true)))

(fn `UserConstructionScript`)